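; BP_Infantry is the infantry unit Blueprint for Toybox Tactics, built on a parent unit class.
; On BeginPlay it loads max health, movement speed and attack range from the Infantry row of DT_UnitClass.
; State changes look up a behavior tree in DT_InfantryOrders, run it via a multicast event and store it as active.
; For BT_Attack, that event also writes the attack target and its location to the blackboard.
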(event `self.ReceiveTick`
  (params (DeltaSeconds :type "Float (single-precision)"))
  (`parent.ReceiveTick` DeltaSeconds))

(event `self.ReceiveActorBeginOverlap`
  (params (OtherActor :type "Actor Object Reference"))
  (`parent.ReceiveActorBeginOverlap` OtherActor))

(event `self.ReceiveBeginPlay`
  (`parent.ReceiveBeginPlay`)
  (bind _returnvalue (`|GetDataTableRow` "/Game/ToyboxTactics/Core/Units/DT_UnitClass.DT_UnitClass" "Infantry")
    (:`then`
      (bind (_health _speed _damage _range) (break `/Game/ToyboxTactics/Core/Units/F_UnitClass` _returnvalue))
      (`HealthComponent.SetMaxHealth` (`self.Health`) _health)
      (set `FloatingPawnMovement.MaxSpeed` (`KismetMathLibrary.Conv_IntToDouble` _speed) (`self.FloatingPawnMovement`))
      (set `self.AttackRange` _range))
    (:`RowNotFound`
      (`KismetSystemLibrary.PrintString` "unit Data not loaded for infantry"))))

(event `ChangeInfantryState`
  (params (NewInfantryState :type Name))
  ;[0.6695 0.244 0.956] Change State Of the infantry
  (bind _returnvalue (`|GetDataTableRow` "/Game/ToyboxTactics/Core/Units/DT_InfantryOrders.DT_InfantryOrders" NewInfantryState)
    (:`then`
      (`/Engine/EditorBlueprintResources/StandardMacros.IsValid` (`AIBlueprintHelperLibrary.GetAIController` self)
        (:`Is Valid`
          (bind _behavoirtree (break `/Game/ToyboxTactics/Core/Units/F_InfantryOrder` _returnvalue))
          (`self.ChangeInfantry_Multicast` _behavoirtree)
          (set `self.Active Behavior` _behavoirtree))))
    (:`RowNotFound`
      (`KismetSystemLibrary.PrintString` "ERROR: New state not found"))))

(event `ChangeInfantry_Multicast`
  (params (Behaviour :type "BehaviorTree Object Reference"))
  (bind _returnvalue (`AIBlueprintHelperLibrary.GetBlackboard` null))
  (bind _attacktarget (`self.AttackTarget`))
  ;[1 1 1] This event should be refactored into the baseclass to prevent DRY coding
  (`AIController.RunBehaviorTree` (`AIBlueprintHelperLibrary.GetAIController` self) Behaviour)
  (if (== Behaviour "/Game/ToyboxTactics/Core/Units/AI/BT_Attack.BT_Attack")
    (`BlackboardComponent.SetValueAsObject` _returnvalue (`self.AttackTargetKeyName`) _attacktarget)
    (`BlackboardComponent.SetValueAsVector` _returnvalue (`self.TargetLocationKeyName`) (`self.K2_GetActorLocation` _attacktarget))))

(fn `UserConstructionScript`
  (`parent.UserConstructionScript`))