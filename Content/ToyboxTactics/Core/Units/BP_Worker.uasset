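; BP_Worker is the worker unit in Toybox Tactics, handling resource mining and construct orders.
; BeginPlay targets the nearest resource node, mainly for testing, then loads health, speed and range from DT_UnitClass.
; Orders set the target node or building, then look up a behavior tree in DT_WorkerOrders and run it through a multicast event.
; Mining uses a looping timer that adds the node's yield to Inventory until nearly full.
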(event `self.ReceiveBeginPlay`
  ;[0 0.9333 1] Set closest resource node as target for worker on beginplay [Mainly for testing purposes]
  (`parent.ReceiveBeginPlay`)
  (bind _outactors (`GameplayStatics.GetAllActorsOfClass` "/Game/ToyboxTactics/BP_ResourceNode.BP_ResourceNode_C"))
  (bind _asbp_resource_node (cast `/Game/ToyboxTactics/BP_ResourceNode` (`.ReturnValue` (`GameplayStatics.FindNearestActor` (`self.K2_GetActorLocation`) _outactors))))
  (set `self.SelectedNode` _asbp_resource_node)
  ;[0.1146 0.6038 0.08177] Fetch Unit Stats
  (bind _returnvalue (`|GetDataTableRow` "/Game/ToyboxTactics/Core/Units/DT_UnitClass.DT_UnitClass" "Worker")
    (:`then`
      (bind (_health _speed _damage _range) (break `/Game/ToyboxTactics/Core/Units/F_UnitClass` _returnvalue))
      (`HealthComponent.SetMaxHealth` (`self.Health`) _health)
      (set `FloatingPawnMovement.MaxSpeed` (`KismetMathLibrary.Conv_IntToDouble` _speed) (`self.FloatingPawnMovement`))
      (set `self.AttackRange` _range))
    (:`RowNotFound`
      (`KismetSystemLibrary.PrintString` "unit Data not loaded for infantry"))))

(event `StartMining`
  ;[1 0.6531 0.1208] Timer to execute the 'Mine Resource' mechanic
  (bind _returnvalue (`KismetSystemLibrary.K2_SetTimerDelegate` (delegate `MiningLoop`) 1.0 true))
  (set `self.MineTimerRefHandler` _returnvalue)
  (set `self.Mining?` true))

(event `MiningLoop`
  ;[1 0.6531 0.1208] Timer to execute the 'Mine Resource' mechanic
  (bind _minedamount (`/Game/ToyboxTactics/BP_ResourceNode.Mine Resource` (`self.SelectedNode`) (`self.MineStrength`)))
  (if (not (< (`self.Inventory`) (- (`self.InventoryMax`) (`self.MineStrength`))))
    (`KismetSystemLibrary.K2_ClearAndInvalidateTimerHandle` (`self.MineTimerRefHandler`))
    (set `self.Mining?` false))
  (set `self.Inventory` (+ _minedamount (`self.Inventory`))))

(event `ChangeState_Worker`
  (params (`New Worker State` :type Name))
  ;[0.7031 0.3247 0.6234] ChangeState event to execute incoming orders
  (`self.SetSelectedActor` `New Worker State`
    (:`Set`
      (bind _returnvalue (`|GetDataTableRow` "/Game/ToyboxTactics/Core/Units/DT_WorkerOrders.DT_WorkerOrders" `New Worker State`)
        (:`then`
          (`/Engine/EditorBlueprintResources/StandardMacros.IsValid` (`AIBlueprintHelperLibrary.GetAIController` self)
            (:`Is Valid`
              (bind _behaviortree (break `/Game/ToyboxTactics/Core/Units/F_WorkerOrder` _returnvalue))
              (`self.ChangeWorker_Multicast` _behaviortree)
              (set `self.Active Behavior` _behaviortree))))
        (:`RowNotFound`
          (`self.ChangeState` (make `/Game/ToyboxTactics/Core/Units/F_ChangeStateData` "NewEnumerator0" null)))))))

(event `ChangeWorker_Multicast`
  (params (Behaviour :type "BehaviorTree Object Reference"))
  (`AIController.RunBehaviorTree` (`AIBlueprintHelperLibrary.GetAIController` self) Behaviour))

(fn `UserConstructionScript`
  (`parent.UserConstructionScript`))