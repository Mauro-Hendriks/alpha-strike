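; BP_DroneUnit is a unit Blueprint that sets its stats from shared unit class data.
; On BeginPlay, after the parent logic, it reads the Worker row of DT_UnitClass and applies Health as max health and Speed as floating pawn max speed.
; A missing row only prints an error, which names infantry rather than drone or worker.
; Construction defers to the parent.
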(event `self.ReceiveBeginPlay`
  (`parent.ReceiveBeginPlay`)
  ;[0 0.9333 1] read unit stats
  (bind _returnvalue (`|GetDataTableRow` "/Game/ToyboxTactics/Core/Units/DT_UnitClass.DT_UnitClass" "Worker")
    (:`then`
      (bind (_health _speed) (break `/Game/ToyboxTactics/Core/Units/F_UnitClass` _returnvalue))
      (`HealthComponent.SetMaxHealth` (`self.Health`) _health)
      (set `FloatingPawnMovement.MaxSpeed` (`KismetMathLibrary.Conv_IntToDouble` _speed) (`self.FloatingPawnMovement`)))
    (:`RowNotFound`
      (`KismetSystemLibrary.PrintString` "unit Data not loaded for infantry"))))

(fn `UserConstructionScript`
  (`parent.UserConstructionScript`))