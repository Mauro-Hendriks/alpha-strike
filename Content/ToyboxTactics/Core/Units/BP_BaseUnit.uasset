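; Base unit for Toybox Tactics, providing selection decals, team ID, orders, attacks, and health bar updates with a red hit flash.
; ChangeState stops attacking, then OrderFilter stores the order's target and routes by unit type; only Worker and Infantry are handled, with Workers also leaving active construction.
; Attack runs a looping timer from DT_AttackData, playing a montage and damaging the target's HealthComponent on both montage start and completion.
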(event `self.ReceiveBeginPlay`
  (`parent.ReceiveBeginPlay`)
  (`SceneComponent.SetVisibility` (`self.SelectionDecal`) false false)
  (`self.ChangeState` (make `/Game/ToyboxTactics/Core/Units/F_ChangeStateData` "NewEnumerator0" self)))

(event `ChangeState`
  (params (ChangeStateData :type "/Game/ToyboxTactics/Core/Units/F_ChangeStateData Structure"))
  (bind (_neworder _orderinitiator _orderclickposition) (break `/Game/ToyboxTactics/Core/Units/F_ChangeStateData` ChangeStateData))
  ;[0.1401 0.375 0.09566] Custom Event that filters the current unit in order to assign the right DataTable for the recieved order.
  (`self.StopAttacking`)
  (`self.Print OrderData in String` _neworder _orderinitiator _orderclickposition)
  (bind _ordername (`self.OrderFilter` _orderinitiator _orderclickposition _neworder)
    (:`Worker`
      (bind _asbp_worker (cast `/Game/ToyboxTactics/Core/Units/BP_Worker` self))
      (if (`/Game/ToyboxTactics/Core/Units/BP_Worker.Constructing?` _asbp_worker)
        (bind _returnvalue (`AddComponent|NODE_AddAC_ConstructionState-0` :`self` (`/Game/ToyboxTactics/Core/Units/BP_Worker.SelectedBuilding` _asbp_worker)))
        (`/Game/ToyboxTactics/Core/Buildings/ActorComponents/AC_ConstructionState.RemoveActiveConstructor` _returnvalue _asbp_worker))
      (`/Game/ToyboxTactics/Core/Units/BP_Worker.ChangeState_Worker` _asbp_worker _ordername))
    (:`Infantry`
      (bind _asbp_infantry (cast `/Game/ToyboxTactics/Core/Units/BP_Infantry` self))
      (`/Game/ToyboxTactics/Core/Units/BP_Infantry.ChangeInfantryState` _asbp_infantry _ordername)
      (`KismetSystemLibrary.PrintString` (`KismetStringLibrary.Conv_NameToString` _ordername)))))

(event `self.AC_SelectableUnit.OnUnitSelected`
  (`SceneComponent.SetVisibility` (`self.SelectionDecal`) true false)
  (`KismetSystemLibrary.PrintString` "Hello"))

(event `Execute Attack Sequence`
  (bind _returnvalue (`self.GetComponentByClass` (`self.AttackTarget`) "/Script/ToyboxTactics.HealthComponent"))
  ;[1 0.07812 0.07812] Attack Targeted Enemy
  (bind _returnvalue_2 (`|GetDataTableRow` "/Game/ToyboxTactics/Core/Units/DT_AttackData.DT_AttackData" (`KismetStringLibrary.Conv_StringToName` (`|GetEnumeratorNameAsString` (`self.UnitType`))))
    (:`then`
      (bind (_damage _attackinterval _animation) (break `/Game/ToyboxTactics/Core/Units/F_AttackData` _returnvalue_2))
      (`|PlayMontage` null _animation
        (:`then`
          _)
        (:`OnCompleted`
          _))
      (`/Engine/EditorBlueprintResources/StandardMacros.IsValid` _returnvalue
        (:`Is Valid`
          (`HealthComponent.ChangeHealth` _returnvalue (`KismetMathLibrary.Conv_IntToDouble` _damage))
          (`KismetSystemLibrary.PrintString` "Attacked for:" true true (struct :`R` 1.0 :`G` 0.117779 :`A` 1.0))
          (`KismetSystemLibrary.PrintString` (`KismetStringLibrary.Conv_IntToString` _damage) true true (struct :`R` 1.0 :`G` 0.062529 :`A` 1.0))
          (`/Engine/EditorBlueprintResources/StandardMacros.IsValid` (`self.AttackTarget`)
            (:`Is Not Valid`
              (`self.StopAttacking`))))))))

(event `self.AC_SelectableUnit.OnUnitDeselected`
  (`SceneComponent.SetVisibility` (`self.SelectionDecal`) false false))

(event `self.Health.OnHealthUpdated`
  (bind _asbp_health_bar (cast `/Game/ToyboxTactics/Core/UI/BP_HealthBar` (`ChildActorComponent.ChildActor` (`self.BP_HealthBar`))))
  (`/Game/ToyboxTactics/Core/UI/BP_HealthBar.UpdateHealthbar` _asbp_health_bar (`HealthComponent.GetNormalizedHealth` (`self.Health`)))
  (bind _returnvalue (`PrimitiveComponent.CreateDynamicMaterialInstance` (`self.StaticMesh`) 1 null "None"))
  (`MaterialInstanceDynamic.SetVectorParameterValue` _returnvalue "ColorTint" (struct :`R` 1.0 :`A` 1.0))
  (`KismetSystemLibrary.Delay` 0.1)
  (`MaterialInstanceDynamic.SetVectorParameterValue` _returnvalue "ColorTint" (struct :`R` 1.0 :`G` 1.0 :`B` 1.0 :`A` 1.0)))

(fn `Attack`
  (bind _returnvalue (`|GetDataTableRow` "/Game/ToyboxTactics/Core/Units/DT_AttackData.DT_AttackData" (`KismetStringLibrary.Conv_StringToName` (`|GetEnumeratorNameAsString` (`self.UnitType`))))
    (:`then`
      (set `self.IsAttacking` true)
      (`KismetSystemLibrary.PrintString` "I AM ATTACKING" true true (struct :`R` 1.0 :`G` 0.072084 :`A` 1.0))
      (bind _returnvalue_2 (`KismetSystemLibrary.K2_SetTimer` null "AttackSequence" (`.AttackInterval_4_6B5993F3435DBF953A24EE9F8FED3EE4` (break `/Game/ToyboxTactics/Core/Units/F_AttackData` _returnvalue)) true))
      (set `self.AttackSeqTimerHandler` _returnvalue_2))
    (:`RowNotFound`
      (`KismetSystemLibrary.PrintString` "ERROR: Attack Data not found." true true (struct :`R` 1.0 :`G` 0.043877 :`B` 0.163586 :`A` 1.0)))))

(fn `AttackSequence`
  (`self.Execute Attack Sequence`))

(fn `GetTeamID`
  (returns (ReturnValue :type Integer))
  (return (`self.TeamID`)))

(fn `StopAttacking`
  (`KismetSystemLibrary.K2_ClearAndInvalidateTimerHandle` (`self.AttackSeqTimerHandler`))
  (set `self.IsAttacking` false))

(fn `UserConstructionScript`
  (`parent.UserConstructionScript`))