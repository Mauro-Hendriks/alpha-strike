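; Actor component that runs a building's construction phase, with build speed scaling with the number of assigned workers.
; StartConstruction swaps the building mesh for a placeholder, reads BuildTime from the building stats DataTable by type and enables Tick.
; Tick counts down by delta time times active workers, then restores the mesh, disables itself and signals completion.
; Workers register and unregister through capped add/remove events; a Nexus worker-spawn branch is left unconnected.
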(event `self.ReceiveBeginPlay`
  (`self.SetComponentTickEnabled` false))

(event `StartConstruction`
  (params (StaticMeshRef :type "StaticMeshComponent Object Reference"))
  ;[0.3851 1 0.4754] gets reference to static mesh and replaces it with a construction mesh. then check building time of specific building in buidling datatable and enables tick event to start buidling process.
  (bind _output_get (set `self.StaticMeshRef` StaticMeshRef))
  (set `self.Building` (`StaticMeshComponent.StaticMesh` StaticMeshRef))
  (`StaticMeshComponent.SetStaticMesh` _output_get "/Game/PolygonScifiWorlds/Meshes/Buildings/SM_Bld_Core_Observation_Greeble_Pipe_Base_01.SM_Bld_Core_Observation_Greeble_Pipe_Base_01")
  (bind _returnvalue (`|GetDataTableRow` "/Game/ToyboxTactics/Core/Buildings/DT_AllBuildingStats.DT_AllBuildingStats" (`KismetStringLibrary.Conv_StringToName` (`|GetEnumeratorNameAsString` (`self.BuildingType`))))
    (:`then`
      (set `self.ConstructionTime` (`.BuildTime` (break `BuildingStats` _returnvalue)))
      (`self.SetComponentTickEnabled` true))
    (:`RowNotFound`
      (`KismetSystemLibrary.PrintText` "Row not found in DataTable"))))

(event `self.ReceiveTick`
  (params (DeltaSeconds :type "Float (single-precision)"))
  (if (not (`self.IsBuild`))
    (bind _output_get (set `self.ConstructionTime` (- (`self.ConstructionTime`) (* DeltaSeconds (`KismetArrayLibrary.Array_Length` (`self.ActiveWorkers`))))))
    (`KismetSystemLibrary.PrintString` (`KismetStringLibrary.Conv_DoubleToString` _output_get) true true (struct :`G` 0.66 :`B` 1.0 :`A` 1.0) 0.0)
    (if (<= _output_get 0.0)
      (`self.SetComponentTickEnabled` false)
      (bind _returnvalue (`StaticMeshComponent.SetStaticMesh` (`self.StaticMeshRef`) (`self.Building`)))
      (set `self.IsBuild` _returnvalue)
      (`self.OnConstructionComplete`))))

(event `AddActiveConstructor`
  (params (worker :type "/Game/ToyboxTactics/Core/Units/BP_Worker Object Reference"))
  (bind _activeworkers (`self.ActiveWorkers`))
  (if (<= (`KismetArrayLibrary.Array_Length` _activeworkers) 7)
    (`KismetArrayLibrary.Array_Add` _activeworkers worker)))

(event `RemoveActiveConstructor`
  (params (Worker :type "/Game/ToyboxTactics/Core/Units/BP_Worker Object Reference"))
  (bind _activeworkers (`self.ActiveWorkers`))
  (if (not (<= (`KismetArrayLibrary.Array_Length` _activeworkers) 0))
    (`KismetArrayLibrary.Array_RemoveItem` _activeworkers Worker)))