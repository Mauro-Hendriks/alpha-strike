(event `self.BuildingMesh.OnComponentBeginOverlap`
  (params (OverlappedComponent :type "PrimitiveComponent Object Reference") (OtherActor :type "Actor Object Reference") (OtherComp :type "PrimitiveComponent Object Reference") (OtherBodyIndex :type Integer) (bFromSweep :type Boolean) (SweepResult :type "HitResult Structure (by ref)"))
  (`/Engine/EditorBlueprintResources/StandardMacros.IsValid` OtherActor
    (:`Is Valid`
      (`KismetArrayLibrary.Array_Add` (`self.Overlap`) OtherActor))))

(event `self.BuildingMesh.OnComponentEndOverlap`
  (params (OverlappedComponent :type "PrimitiveComponent Object Reference") (OtherActor :type "Actor Object Reference") (OtherComp :type "PrimitiveComponent Object Reference") (OtherBodyIndex :type Integer))
  (`/Engine/EditorBlueprintResources/StandardMacros.IsValid` OtherActor
    (:`Is Valid`
      (`KismetArrayLibrary.Array_RemoveItem` (`self.Overlap`) OtherActor))))

(event `OnBulidUnit`
  (params (`Unit Type` :type "/Game/ToyboxTactics/Core/Units/E_UnitTypes Enum" :default "NewEnumerator0"))
  ;[1 1 1] Adds the unit to the training queue and starts training the unit
  (if (`KismetArrayLibrary.Array_Contains` (`self.Trainable Unit Types`) `Unit Type`)
    (if (`/Game/ToyboxTactics/Core/Buildings/ActorComponents/AC_ConstructionState.IsBuild` (`self.AC_ConstructionState`))
      (switch `/Game/ToyboxTactics/Core/Units/E_UnitTypes` `Unit Type`
        (:`NewEnumerator0`
          (bind _asactor (castclass `Actor` "/Game/ToyboxTactics/Core/Units/BP_Worker.BP_Worker_C"))
          (`self.AddTroopsToLine` _asactor))
        (:`NewEnumerator1`
          (bind _asactor_2 (castclass `Actor` "/Game/ToyboxTactics/Core/Units/BP_Infantry.BP_Infantry_C"))
          (`self.AddTroopsToLine` _asactor_2))
        (:`NewEnumerator2`
          (bind _asactor_3 (castclass `Actor` "/Game/ToyboxTactics/Core/Units/BP_Healer.BP_Healer_C"))
          (`self.AddTroopsToLine` _asactor_3))
        (:`NewEnumerator3`
          (bind _asactor_4 (castclass `Actor` "/Game/ToyboxTactics/Core/Units/BP_Heavy.BP_Heavy_C"))
          (`self.AddTroopsToLine` _asactor_4))
        (:`NewEnumerator4`
          (bind _asactor_5 (castclass `Actor` "/Game/ToyboxTactics/Core/Units/BP_DroneUnit.BP_DroneUnit_C"))
          (`self.AddTroopsToLine` _asactor_5))))))

(event `TrainTroop`
  ;[0.1429 0.7681 1] casts to blueprint of unit who is first in line, then looks for specific unit in datatable to start training that unit with his own training time
  (if (not (`self.Training`))
    (set `self.Training` true)
    (bind _asbp_base_unit (castclass `/Game/ToyboxTactics/Core/Units/BP_BaseUnit` (`|GetArrayItem` (`self.TroopsToTrain`))))
    (set `self.NextUnitToSpawn` _asbp_base_unit)
    (bind _output_get (set `self.UnitType` (`.UnitType` (defaults `Object` _asbp_base_unit))))
    (bind _returnvalue (`|GetDataTableRow` "/Game/ToyboxTactics/Core/Units/DT_UnitClass.DT_UnitClass" (`KismetStringLibrary.Conv_StringToName` (`|GetEnumeratorNameAsString` _output_get)))
      (:`then`
        (set `self.TrainTimeOfCurrentUnit` (`KismetMathLibrary.Conv_IntToDouble` (`.TrainingTime_17_D1D597E9499471F5C7E7E59E5431A2C2` (break `/Game/ToyboxTactics/Core/Units/F_UnitClass` _returnvalue))))
        (`self.SetActorTickEnabled` true)))))

(event `self.ReceiveTick`
  (params (DeltaSeconds :type "Float (single-precision)"))
  ;[0.8845 0.4662 1] counts down from training time. when 0, spawns unit and checks if there are more units in list. if so, continues training.
  (bind _multiplier (`self.Get Train Speed Multiplier`))
  (bind _output_get (set `self.TrainTimeOfCurrentUnit` (- (`self.TrainTimeOfCurrentUnit`) (* DeltaSeconds _multiplier))))
  (`KismetSystemLibrary.PrintString` (`KismetStringLibrary.Conv_DoubleToString` _output_get) true true (struct :`R` 1.0 :`G` 0.163231 :`A` 1.0) 0.0)
  (if (<= _output_get 0.0)
    (`self.SetActorTickEnabled` false)
    (`/Game/ToyboxTactics/Core/Buildings/ActorComponents/AC_ActorSpawner.SpawnActor` (`self.AC_ActorSpawner`) (`self.NextUnitToSpawn`) (`SceneComponent.K2_GetComponentToWorld` (`self.UnitSpawnPoint`)) (`self.TeamID`))
    (`KismetArrayLibrary.Array_Remove` (`self.TroopsToTrain`))
    (if (> (`KismetArrayLibrary.Array_Length` (`self.TroopsToTrain`)) 0)
      (set `self.Training` false)
      (`self.TrainTroop`)
      (else
        (set `self.Training` false)))))

(event `self.AC_SelectableUnitComponent.OnUnitSelected`
  (`KismetSystemLibrary.PrintString` "Building Selected"))

(fn `Get Train Speed Multiplier`
  (returns (Multiplier :type "Float (double-precision)"))
  (return 1.0))

(fn `UserConstructionScript`)