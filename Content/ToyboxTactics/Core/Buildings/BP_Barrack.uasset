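; BP_Barrack is the Toybox Tactics barracks building that queues units for training.
; It disables tick on BeginPlay and hands construction to ACConstructionState with its building mesh once the construction state change fires.
; Number keys 1 to 5 each pass a unit type to OnBulidUnit.
; Its train speed multiplier equals the team's barracks count from the game mode, with a minimum of one.
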(event `self.ReceiveBeginPlay`
  ;[1 1 1] dissables tick event
  (`self.SetActorTickEnabled` false))

(event `self.ChangeBuildingStateToConstruction`
  ;[1 1 1] starts construction after building is placed
  (`self.Start Construction`))

(event `Start Construction`
  ;[1 1 1] starts construction after building is placed
  (`/Game/ToyboxTactics/Core/Buildings/ActorComponents/AC_ConstructionState.StartConstruction` (`self.AC_ConstructionState`) (`self.BuildingMesh`)))

(event `Key|One`
  (params (Key :type "Key Structure"))
  ;[0.6927 0 0] checks if barracks is build and starts macro wich adds choosen unit to list
  (:`Pressed`
    (`self.OnBulidUnit` "NewEnumerator1")))

(event `Key|Two`
  (params (Key :type "Key Structure"))
  ;[0.6927 0 0] checks if barracks is build and starts macro wich adds choosen unit to list
  (:`Pressed`
    (`self.OnBulidUnit` "NewEnumerator3")))

(event `Key|Three`
  (params (Key :type "Key Structure"))
  ;[0.6927 0 0] checks if barracks is build and starts macro wich adds choosen unit to list
  (:`Pressed`
    (`self.OnBulidUnit` "NewEnumerator4")))

(event `Key|Four`
  (params (Key :type "Key Structure"))
  ;[0.6927 0 0] checks if barracks is build and starts macro wich adds choosen unit to list
  (:`Pressed`
    (`self.OnBulidUnit` "NewEnumerator2")))

(event `Key|Five`
  (params (Key :type "Key Structure"))
  ;[0.6927 0 0] checks if barracks is build and starts macro wich adds choosen unit to list
  (:`Pressed`
    (`self.OnBulidUnit` "NewEnumerator0")))

(fn `Get Train Speed Multiplier`
  (returns (Multiplier :type "Float (double-precision)"))
  (return (`KismetMathLibrary.Conv_IntToDouble` (`KismetMathLibrary.Max` (`KismetArrayLibrary.Array_Length` (`.TeamBaracks_10_F636DC29494FD60CD492B180E3C7181A` (break `/Game/ToyboxTactics/Core/F_BuildingsList` (`BlueprintMapLibrary.Map_Find` (`/Game/ToyboxTactics/Core/BP_TTGameMode.TeamsBuildings` (cast `/Game/ToyboxTactics/Core/BP_TTGameMode` (`GameplayStatics.GetGameMode`) :!pure true)) (`self.TeamID`))))) 1))))

(fn `UserConstructionScript`
  (`parent.UserConstructionScript`))