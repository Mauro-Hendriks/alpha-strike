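; BP_Nexus is a building in Toybox Tactics that spawns a worker unit when its construction finishes.
; ChangeBuildingStatetoConstruction hands the building mesh to the construction state component to start construction.
; The component's completion event calls SpawnWorker, which has the actor spawner component create a BP_Worker at UnitSpawnPoint with a hard-coded team ID.
; BeginPlay is empty, and a player ID debug print is left unconnected.
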(event `self.ReceiveBeginPlay`)

(event `SpawnWorker`
  (`/Game/ToyboxTactics/Core/Buildings/ActorComponents/AC_ActorSpawner.SpawnActor` (`self.AC_ActorSpawner`) "/Game/ToyboxTactics/Core/Units/BP_Worker.BP_Worker_C" (`SceneComponent.K2_GetComponentToWorld` (`self.UnitSpawnPoint`)) 0))

(event `self.ChangeBuildingStateToConstruction`
  (`/Game/ToyboxTactics/Core/Buildings/ActorComponents/AC_ConstructionState.StartConstruction` (`self.AC_ConstructionState`) (`self.BuildingMesh`)))

(event `self.AC_ConstructionState.OnConstructionComplete`
  (`self.SpawnWorker`))

(fn `UserConstructionScript`
  (`parent.UserConstructionScript`))