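; Desktop HUD that shows a unit-training menu at a clicked building in Toybox Tactics.
; On BeginPlay it spawns a BP_BuildingUnitUI actor that hosts the widget.
; Clicking a finished building moves that actor to the building, initializes its buttons for the building type and makes the widget visible.
; Deselecting the building collapses the widget.
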(event `self.ReceiveBeginPlay`
  ;[1 1 1] Spawn widget blueprint container actor
  (bind _returnvalue (`|SpawnActorFromClass` "/Game/ToyboxTactics/Core/UI/BP_BuildingUnitUI.BP_BuildingUnitUI_C" (`self.GetTransform`) "Undefined" "MultiplyWithRoot" null null))
  (set `self.Building Unit UI` _returnvalue))

(event `OnBuildingClicked`
  (params (`Clicked Building` :type "/Game/ToyboxTactics/Core/Buildings/BP_buildingBase Object Reference"))
  ;[1 1 1] Set the building unit train menu to the buildings location and enable the widget
  (if (`/Game/ToyboxTactics/Core/Buildings/ActorComponents/AC_ConstructionState.IsBuild` (`/Game/ToyboxTactics/Core/Buildings/BP_buildingBase.AC_ConstructionState` `Clicked Building`))
    (`self.K2_SetActorLocation` (`self.Building Unit UI`) (`self.K2_GetActorLocation` `Clicked Building`) false false)
    (`/Game/ToyboxTactics/Core/UI/BP_BuildingUnitUI.Initialize Buttons` (`self.Building Unit UI`) (`BaseBuilding.BuildingType` `Clicked Building`) `Clicked Building`)
    (set `Widget.Visibility` "Visible" (`WidgetComponent.GetWidget` (`/Game/ToyboxTactics/Core/UI/BP_BuildingUnitUI.Widget Actor` (`self.Building Unit UI`))))))

(event `OnBuldingDeselected`
  ;[1 1 1] Disable the unit train widget
  (set `Widget.Visibility` "Collapsed" (`WidgetComponent.GetWidget` (`/Game/ToyboxTactics/Core/UI/BP_BuildingUnitUI.Widget Actor` (`self.Building Unit UI`)))))

(fn `UserConstructionScript`)