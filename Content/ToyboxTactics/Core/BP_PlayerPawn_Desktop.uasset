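; Desktop player pawn for an RTS-style game, handling camera control, build menu toggling and orders to selected units.
; Enhanced Input drives yaw-relative movement, spring-arm zoom and the menu; mouse edge-scroll functions exist but are disconnected.
; OrderUnitEvent traces under the cursor for an AC_UnitOrderGenerator, which picks an order from the target's faction (TeamID versus PlayerId).
; Each selected unit then has its FloatingPawnMovement deactivated and receives the order through ChangeState.
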(event `self.ReceiveBeginPlay`
  ;[1 1 1] Sets visibilty for video at the start of the game and adds mapping context for enhanced input on game start
  (`SceneComponent.SetVisibility` (`self.Widget`) (`self.bBuildMenuVisible`) false)
  (message `EnhancedInputSubsystemInterface.AddMappingContext` (pcsubsystem `EnhancedInputLocalPlayerSubsystem` (`GameplayStatics.GetPlayerController` 0)) "/Game/ToyboxTactics/Input/IMC_Default.IMC_Default" 0 (struct)))

(event `self.OrderUnitEvent`
  ;[1 1 1] Check if we're hitting an object implementing a UnitOrderGenerator Component
  (bind (_ordergenerator _hitactor _impactpoint) (`self.GetOrderGenerator`))
  (`/Engine/EditorBlueprintResources/StandardMacros.IsValid` _ordergenerator
    (:`Is Valid`
      (bind _returnvalue (`self.GetAssociatedFaction` _hitactor))
      (bind _neworder (`/Game/ToyboxTactics/Core/AC_UnitOrderGenerator.GetOrder` _ordergenerator _returnvalue))
      (`self.PassNewOrderToSelectedUnits` (make `/Game/ToyboxTactics/Core/Units/F_ChangeStateData` _neworder _hitactor _impactpoint)))))

(event `WhenButtonClicked`
  ;[1 1 1] Check if we're hitting an object implementing a UnitOrderGenerator Component
)

(event `self.ReceiveTick`
  (params (DeltaSeconds :type "Float (single-precision)"))
  ;[1 1 1] MouseCameraMovement, for now disabled for easier debugging
)

(event `EnhancedInput|/Game/ToyboxTactics/Input/InputActions/IA_Zoom`
  (params (ActionValue :type "Float (double-precision)") (ElapsedSeconds :type "Float (double-precision)") (TriggeredSeconds :type "Float (double-precision)") (InputAction :type "InputAction Object Reference" :default "/Game/ToyboxTactics/Input/InputActions/IA_Zoom.IA_Zoom"))
  (bind (_zoombound_x _zoombound_y) (`KismetMathLibrary.BreakVector2D` (`self.ZoomBound`)))
  ;[1 1 1] MouseZoom
  (:`Triggered`
    (set `SpringArmComponent.TargetArmLength` (`KismetMathLibrary.FClamp` (+ (`SpringArmComponent.TargetArmLength` (`self.SpringArm`)) (* ActionValue (`self.ZoomSpeed`))) _zoombound_x _zoombound_y) (`self.SpringArm`))))

(event `EnhancedInput|/Game/ToyboxTactics/Input/InputActions/IA_BuildingList`
  (params (ActionValue :type Boolean) (ElapsedSeconds :type "Float (double-precision)") (TriggeredSeconds :type "Float (double-precision)") (InputAction :type "InputAction Object Reference" :default "/Game/ToyboxTactics/Input/InputActions/IA_BuildingList.IA_BuildingList"))
  ;[1 1 1] Open/Close BuildingList
  (:`Started`
    (bind _output_get (set `self.bBuildMenuVisible` (not (`self.bBuildMenuVisible`))))
    (`SceneComponent.SetVisibility` (`self.Widget`) _output_get false)
    (`WidgetBlueprintLibrary.SetInputMode_GameAndUIEx` (`GameplayStatics.GetPlayerController` 0) (`WidgetComponent.GetUserWidgetObject` (`self.Widget`)))))

(event `EnhancedInput|/Game/IA_MoveCamera`
  (params (ActionValue :type "Vector2D Structure") (ElapsedSeconds :type "Float (double-precision)") (TriggeredSeconds :type "Float (double-precision)") (InputAction :type "InputAction Object Reference" :default "/Game/IA_MoveCamera.IA_MoveCamera"))
  (bind (_returnvalue_roll _returnvalue_pitch _returnvalue_yaw) (`KismetMathLibrary.BreakRotator` (`self.K2_GetActorRotation`)))
  (bind (_returnvalue_roll_2 _returnvalue_pitch_2 _returnvalue_yaw_2) (`KismetMathLibrary.BreakRotator` (`self.K2_GetActorRotation`)))
  ;[1 1 1] Camera Movement
  (:`Triggered`
    (`self.AddMovementInput` (`KismetMathLibrary.GetForwardVector` (`KismetMathLibrary.MakeRotator` 0.0 0.0 _returnvalue_yaw)) ActionValue_Y)
    (`self.AddMovementInput` (`KismetMathLibrary.GetRightVector` (`KismetMathLibrary.MakeRotator` _returnvalue_roll_2 0.0 _returnvalue_yaw_2)) ActionValue_X)))

(fn `GetAssociatedFaction`
  (params (HitActor :type "Actor Object Reference"))
  (returns (ReturnValue :type "/Game/ToyboxTactics/Core/E_FactionType Enum"))
  (bind _asbp_base_unit (cast `/Game/ToyboxTactics/Core/Units/BP_BaseUnit` HitActor)
    (:`then`
      (return (select `bool` (== (`/Game/ToyboxTactics/Core/Units/BP_BaseUnit.TeamID` _asbp_base_unit) (`PlayerState.PlayerId` (`Controller.PlayerState` (`GameplayStatics.GetPlayerController` 0)))) :`false` "NewEnumerator1" :`true` "NewEnumerator0" :!type "/Game/ToyboxTactics/Core/E_FactionType Enum")))
    (:`CastFailed`
      (bind _asbase_building (cast `BaseBuilding` HitActor)
        (:`then`
          (return (select `bool` (== (`BaseBuilding.TeamID` _asbase_building) (`PlayerState.PlayerId` (`Controller.PlayerState` (`GameplayStatics.GetPlayerController` 0)))) :`false` "NewEnumerator1" :`true` "NewEnumerator0" :!type "/Game/ToyboxTactics/Core/E_FactionType Enum")))
        (:`CastFailed`
          (return "NewEnumerator2"))))))

(fn `GetOrderGenerator`
  (returns (OrderGenerator :type "/Game/ToyboxTactics/Core/AC_UnitOrderGenerator Object Reference") (HitActor :type "Actor Object Reference") (ImpactPoint :type "Vector Structure"))
  (bind (_hitresult _returnvalue) (`PlayerController.GetHitResultUnderCursorByChannel` (`self.GetLocalViewingPlayerController`) "TraceTypeQuery1" true))
  (bind (_bblockinghit _binitialoverlap _time _distance _location _impactpoint _normal _impactnormal _physmat _hitactor) (`GameplayStatics.BreakHitResult` _hitresult))
  (if _returnvalue
    (return (`self.GetComponentByClass` _hitactor "/Game/ToyboxTactics/Core/AC_UnitOrderGenerator.AC_UnitOrderGenerator_C") _hitactor _impactpoint)))

(fn `MoveDown`
  (bind (_returnvalue_x _returnvalue_y) (`KismetMathLibrary.BreakVector2D` (`WidgetLayoutLibrary.GetViewportSize`)))
  (bind _returnvalue (`WidgetLayoutLibrary.GetMousePositionOnViewport`))
  (bind (_returnvalue_x_2 _returnvalue_y_2) (`KismetMathLibrary.BreakVector2D` (* _returnvalue (`WidgetLayoutLibrary.GetViewportScale`))))
  (`SceneComponent.K2_AddRelativeLocation` (`self.DefaultSceneRoot`) (* (-1.0 0.0 0.0) (`KismetMathLibrary.FClamp` (`KismetMathLibrary.NormalizeToRange` _returnvalue_y_2 (* _returnvalue_y 0.95) _returnvalue_y)) (`self.CameraMovementSpeed`)) false false))

(fn `MoveLeft`
  (bind _returnvalue_x (`KismetMathLibrary.BreakVector2D` (`WidgetLayoutLibrary.GetViewportSize`)))
  (bind _returnvalue (`WidgetLayoutLibrary.GetMousePositionOnViewport`))
  (bind _returnvalue_x_2 (`KismetMathLibrary.BreakVector2D` (* _returnvalue (`WidgetLayoutLibrary.GetViewportScale`))))
  (`SceneComponent.K2_AddRelativeLocation` (`self.DefaultSceneRoot`) (* (0.0 -1.0 0.0) (- 1.0 (`KismetMathLibrary.FClamp` (`KismetMathLibrary.NormalizeToRange` _returnvalue_x_2 0.0 (* _returnvalue_x 0.05)))) (`self.CameraMovementSpeed`)) false false))

(fn `MoveRight`
  (bind _returnvalue_x (`KismetMathLibrary.BreakVector2D` (`WidgetLayoutLibrary.GetViewportSize`)))
  (bind _returnvalue (`WidgetLayoutLibrary.GetMousePositionOnViewport`))
  (bind _returnvalue_x_2 (`KismetMathLibrary.BreakVector2D` (* _returnvalue (`WidgetLayoutLibrary.GetViewportScale`))))
  (`SceneComponent.K2_AddRelativeLocation` (`self.DefaultSceneRoot`) (* (0.0 1.0 0.0) (`KismetMathLibrary.FClamp` (`KismetMathLibrary.NormalizeToRange` _returnvalue_x_2 (* _returnvalue_x 0.95) _returnvalue_x)) (`self.CameraMovementSpeed`)) false false))

(fn `MoveUp`
  (bind _returnvalue_x (`KismetMathLibrary.BreakVector2D` (`WidgetLayoutLibrary.GetViewportSize`)))
  (bind _returnvalue (`WidgetLayoutLibrary.GetMousePositionOnViewport`))
  (bind (_returnvalue_x_2 _returnvalue_y) (`KismetMathLibrary.BreakVector2D` (* _returnvalue (`WidgetLayoutLibrary.GetViewportScale`))))
  (`SceneComponent.K2_AddRelativeLocation` (`self.DefaultSceneRoot`) (* (1.0 0.0 0.0) (- 1.0 (`KismetMathLibrary.FClamp` (`KismetMathLibrary.NormalizeToRange` _returnvalue_y 0.0 (* _returnvalue_x 0.05)))) (`self.CameraMovementSpeed`)) false false))

(fn `PassNewOrderToSelectedUnits`
  (params (ChangeStateData :type "/Game/ToyboxTactics/Core/Units/F_ChangeStateData Structure"))
  (bind _returnvalue (`SelectedUnitsListComponent.GetCurrentlySelectedUnits` (`self.SelectedUnitListComponent`)))
  (for _array_element _returnvalue
    (bind _asbp_base_unit (cast `/Game/ToyboxTactics/Core/Units/BP_BaseUnit` (`ActorComponent.GetOwner` _array_element)))
    (`ActorComponent.SetActive` (`/Game/ToyboxTactics/Core/Units/BP_BaseUnit.FloatingPawnMovement` _asbp_base_unit) false false)
    (`/Game/ToyboxTactics/Core/Units/BP_BaseUnit.ChangeState` _asbp_base_unit (`local.ChangeStateData`))))

(fn `UserConstructionScript`)