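; Game mode for Toybox Tactics that tracks each team's nexuses and barracks and triggers defeat.
; Building create and destroy events update per-team struct lists in a TeamID-keyed map, though barrack removal always reads team 0's entry.
; When a team's last nexus dies, every logged-in controller's player state receives PlayerLosses with that TeamID.
; BeginPlay also caches the building-radius components of all placed nexuses.
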(event `self.CreatedBuilding`
  (params (NewBuilding :type "BaseBuilding Object Reference") (TeamID :type Integer))
  ;[1 1 1] When a building is created look if its the nexus or barrack then called the create event
  (bind _asbp_nexus (cast `/Game/ToyboxTactics/Core/Buildings/BP_Nexus` NewBuilding)
    (:`then`
      (`self.CreatedNexus` _asbp_nexus TeamID))
    (:`CastFailed`
      (bind _asbp_barrack (cast `/Game/ToyboxTactics/Core/Buildings/BP_Barrack` NewBuilding))
      (`self.CreatedBarrack` _asbp_barrack TeamID))))

(event `self.DestroyedBuilding`
  (params (DestroyedBuilding :type "BaseBuilding Object Reference") (TeamID :type Integer))
  ;[1 1 1] when building is destroyed loof its the nexus or barrack then called the killed event
  (bind _asbp_nexus (cast `/Game/ToyboxTactics/Core/Buildings/BP_Nexus` DestroyedBuilding)
    (:`then`
      (`self.KilledNexus` _asbp_nexus TeamID))
    (:`CastFailed`
      (bind _asbp_barrack (cast `/Game/ToyboxTactics/Core/Buildings/BP_Barrack` DestroyedBuilding))
      (`self.KilledBarrack` _asbp_barrack TeamID))))

(event `self.K2_PostLogin`
  (params (NewPlayer :type "PlayerController Object Reference"))
  ;[1 1 1] Set new player in a list
  (`KismetArrayLibrary.Array_Add` (`self.AllPlayerControllers`) NewPlayer))

(event `CreatedNexus`
  (params (`New Nexus` :type "/Game/ToyboxTactics/Core/Buildings/BP_Nexus Object Reference") (`Team ID` :type Integer))
  (bind _value (`BlueprintMapLibrary.Map_Find` (`self.TeamsBuildings`) `Team ID`))
  ;[1 1 1] When a nexus is created look if the TeamID is a map key if its not make a new map with the team id and new nexus.
  ; If there exist a key thats the same as the TeamID then get the list out of the struct and set it as a temp variable to hold the list. Then add the new nexus to that list and set it as a struct then replace the old struct with the new struct.
  (if (`BlueprintMapLibrary.Map_Contains` (`self.TeamsBuildings`) `Team ID`)
    (bind _output_get (set `self.Team Nexuses` (`.TeamNexuses_4_1B06119A45050A45940DA68D930885C3` (break `/Game/ToyboxTactics/Core/F_BuildingsList` _value))))
    (`KismetArrayLibrary.Array_Add` _output_get `New Nexus`)
    (bind _structout (setmembers `/Game/ToyboxTactics/Core/F_BuildingsList` :`StructRef` _value :`TeamNexuses` (`self.Team Nexuses`)))
    (`BlueprintMapLibrary.Map_Add` (`self.TeamsBuildings`) `Team ID` _structout)
    (else
      (`BlueprintMapLibrary.Map_Add` (`self.TeamsBuildings`) `Team ID` (make `/Game/ToyboxTactics/Core/F_BuildingsList` (`|MakeArray` `New Nexus`))))))

(event `KilledNexus`
  (params (`Killed Nexus` :type "/Game/ToyboxTactics/Core/Buildings/BP_Nexus Object Reference") (`Team ID` :type Integer))
  (bind (_value _returnvalue) (`BlueprintMapLibrary.Map_Find` (`self.TeamsBuildings`) `Team ID`))
  ;[1 1 1] When a nexus remove the corresponding nexus. and when nexus list is empty the player with that ID loses
  (if _returnvalue
    (bind _output_get (set `self.Team Nexuses` (`.TeamNexuses_4_1B06119A45050A45940DA68D930885C3` (break `/Game/ToyboxTactics/Core/F_BuildingsList` _value))))
    (`KismetArrayLibrary.Array_RemoveItem` _output_get `Killed Nexus`)
    (bind _structout (setmembers `/Game/ToyboxTactics/Core/F_BuildingsList` :`StructRef` _value :`TeamNexuses` (`self.Team Nexuses`)))
    (`BlueprintMapLibrary.Map_Add` (`self.TeamsBuildings`) `Team ID` _structout)
    (if (`KismetArrayLibrary.Array_IsEmpty` (`self.Team Nexuses`))
      (for _array_element (`self.AllPlayerControllers`)
        (bind _asbp_player_state (cast `/Game/ToyboxTactics/Core/BP_PlayerState` (`Controller.PlayerState` _array_element)))
        (`/Game/ToyboxTactics/Core/BP_PlayerState.PlayerLosses` _asbp_player_state `Team ID`)))))

(event `CreatedBarrack`
  (params (`New Barrack` :type "/Game/ToyboxTactics/Core/Buildings/BP_Barrack Object Reference") (`Team ID` :type Integer))
  (bind _value (`BlueprintMapLibrary.Map_Find` (`self.TeamsBuildings`) `Team ID`))
  ;[1 1 1] When a Barrack is created ladd it to the team barrack.
  (if (`BlueprintMapLibrary.Map_Contains` (`self.TeamsBuildings`) `Team ID`)
    (bind _output_get (set `self.Team Baracks` (`.TeamBaracks_10_F636DC29494FD60CD492B180E3C7181A` (break `/Game/ToyboxTactics/Core/F_BuildingsList` _value))))
    (`KismetArrayLibrary.Array_Add` _output_get `New Barrack`)
    (bind _structout (setmembers `/Game/ToyboxTactics/Core/F_BuildingsList` :`StructRef` _value :`TeamBaracks` (`self.Team Baracks`)))
    (`BlueprintMapLibrary.Map_Add` (`self.TeamsBuildings`) `Team ID` _structout)))

(event `KilledBarrack`
  (params (`Killed Barrack` :type "/Game/ToyboxTactics/Core/Buildings/BP_Barrack Object Reference") (`Team ID` :type Integer))
  (bind (_value _returnvalue) (`BlueprintMapLibrary.Map_Find` (`self.TeamsBuildings`)))
  ;[1 1 1] When a barrack is removed, remove the corresponding barack.
  (if _returnvalue
    (bind _output_get (set `self.Team Baracks` (`.TeamBaracks_10_F636DC29494FD60CD492B180E3C7181A` (break `/Game/ToyboxTactics/Core/F_BuildingsList` _value))))
    (`KismetArrayLibrary.Array_RemoveItem` _output_get `Killed Barrack`)
    (bind _structout (setmembers `/Game/ToyboxTactics/Core/F_BuildingsList` :`StructRef` _value :`TeamBaracks` (`self.Team Baracks`)))
    (`BlueprintMapLibrary.Map_Add` (`self.TeamsBuildings`) `Team ID` _structout)))

(event `self.ReceiveBeginPlay`
  (bind _outactors (`GameplayStatics.GetAllActorsOfClass` "/Game/ToyboxTactics/Core/Buildings/BP_Nexus.BP_Nexus_C"))
  (for _array_element _outactors
    (`KismetArrayLibrary.Array_Add` (`self.AllBuildingComponents`) (`/Game/ToyboxTactics/Core/Buildings/BP_Nexus.BuildingRadius` _array_element))))

(fn `UserConstructionScript`)