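; BP_ResourceNode is a Toybox Tactics resource node that holds a finite amount to be mined and destroys itself when depleted.
; MineResource clamps the requested amount to what remains, subtracts it, fires the OnResourceMined dispatcher and returns the amount actually collected.
; The node binds its own handler to that dispatcher at BeginPlay, so the depletion check and destruction run as a reaction to each mining call.
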(event `self.ReceiveBeginPlay`
  ;[1 1 1] Setup event binding for mining. The mining itself is called via a function
  (add `self.OnResourceMined` (delegate `ResourceMined`)))

(event `ResourceMined`
  ;[1 1 1] Setup event binding for mining. The mining itself is called via a function
  (if (<= (`self.ResourceRemaining`) 0)
    (`self.K2_DestroyActor`)))

(fn `CalculateCollectAmount`
  (params (CollectAmount :type Integer))
  (returns (CollectedAmount :type Integer))
  (return (select `bool` (< (`self.ResourceRemaining`) CollectAmount) :`false` CollectAmount :`true` (`self.ResourceRemaining`))))

(fn `Mine Resource`
  (params (MineAmount :type Integer))
  (returns (MinedAmount :type Integer))
  (bind _collectedamount (`self.CalculateCollectAmount` MineAmount))
  (set `self.ResourceRemaining` (- (`self.ResourceRemaining`) _collectedamount))
  (`self.OnResourceMined`)
  (return _collectedamount))

(fn `UserConstructionScript`)